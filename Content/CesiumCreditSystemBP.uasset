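; Cesium credit system actor Blueprint that shows data credits on screen through a screen credits widget.
; On BeginPlay it creates the widget, adds it to the viewport and starts it with empty HTML and a blank browser page.
; Each Tick where CreditsUpdated is set, it copies DisplayCredits to the widget and, if enabled, pushes the full and on-screen credit HTML.
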(event EventBeginPlay
  (|CallParentFunction)
  (bind _returnvalue (UserInterface|CreateWidget "/CesiumForUnreal/ScreenCredits.ScreenCredits_C"))
  (bind _output_get (Variables|Default|SetScreenCreditsObj _returnvalue))
  (Default|UpdateHtml _output_get)
  (UserInterface|Viewport|AddtoViewport _output_get 0)
  (Class|WebBrowser|LoadURL (Variables|/CesiumForUnreal/ScreenCredits.ScreenCredits_C|GetWebBrowser_52 (Variables|Default|GetScreenCreditsObj)) "about:blank"))

(event Collision|EventActorBeginOverlap
  (params (OtherActor :type Actor%20Object%20Reference)))

(event EventTick
  (params (DeltaSeconds :type Float%20%28single-precision%29))
  (|CallParentFunction DeltaSeconds)
  (if (Variables|Default|GetCreditsUpdated)
    (bind _output_get (Variables|/CesiumForUnreal/ScreenCredits.ScreenCredits_C|SetDisplayCredits (Variables|Default|GetScreenCreditsObj) (Variables|Default|GetDisplayCredits)))
    (if _output_get
      (Default|UpdateHtml (Variables|Default|GetScreenCreditsObj) (Variables|Default|GetCredits))
      (Default|UpdateOn-ScreenHtml (Variables|Default|GetScreenCreditsObj) (Variables|Default|GetOnScreenCredits)))))

(fn ConstructionScript)